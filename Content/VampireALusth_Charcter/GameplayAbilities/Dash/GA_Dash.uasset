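; GA_Dash is a gameplay ability that launches the BP_VAl character forward through pawns, damaging and knocking back those it hits.
; On activation it commits, starts the UI cooldown, zeroes ground friction, applies a forward impulse, sets pawn collision to overlap and plays the dash montage.
; A gameplay event supplies the target for damage, then pushes and stuns it if it is a BP_VAl.
; Montage end or interruption restores friction and blocking collision.
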(event `self.K2_ActivateAbility`
  (`self.K2_CommitAbility`)
  (`self.DoUICooldown`)
  (bind _asbp_val (cast `/Game/ThirdPerson/Blueprints/BP_VAl` (`self.GetOwningActorFromActorInfo`))
    (:`then`
      (set `self.OriginalGroundFrictionFromBP_VAL` (`/Game/ThirdPerson/Blueprints/BP_VAl.OriginalGroundFriction` _asbp_val))
      (bind _charactermovement (`Character.CharacterMovement` _asbp_val))
      (set `CharacterMovementComponent.GroundFriction` 0.0 _charactermovement)
      (`CharacterMovementComponent.AddImpulse` _charactermovement (* (`Actor.GetActorForwardVector` _asbp_val) (`self.ImpulseValue`)) true)
      (bind _characterbase (`self.Get Player Character and Controller`))
      (`/Game/ThirdPerson/Blueprints/BP_VAl.SetCollisionToPawn` _characterbase "ECR_Overlap")
      (`AbilityTask_PlayMontageAndWait.CreatePlayMontageAndWaitProxy` "None" "/Game/VampireALusth_Charcter/Animation/AM_Dash_VAL.AM_Dash_VAL" 0.5
        (:`then`
          (bind (_asynctaskproxy _payload) (`AbilityTask_WaitGameplayEvent.WaitGameplayEvent` (struct :`TagName` "skill.dash.dealDamage") null)
            (:`EventReceived`
              (bind (_eventtag _instigator _target) (break `GameplayEventData` _payload))
              (`self.BP_ApplyGameplayEffectToTarget` (`AbilitySystemBlueprintLibrary.AbilityTargetDataFromActor` _target) "/Game/VampireALusth_Charcter/GameplayAbilities/Dash/GE_DashDamage.GE_DashDamage_C")
              (bind _asbp_val_2 (cast `/Game/ThirdPerson/Blueprints/BP_VAl` _target))
              (`/Game/ThirdPerson/Blueprints/BP_VAl.PushCharacter` _asbp_val_2 (`KismetMathLibrary.Normal` (- (`Actor.K2_GetActorLocation` _asbp_val_2) (`Actor.K2_GetActorLocation` (`self.GetOwningActorFromActorInfo`)))) 4000.0 2.0 "/Game/VampireALusth_Charcter/Animation/AM_GroundBlast_InAir.AM_GroundBlast_InAir")
              (`Character.PlayAnimMontage` _asbp_val_2 "/Game/VampireALusth_Charcter/Animation/AM_GroundBlast_StandUp.AM_GroundBlast_StandUp" 1.0 "None"))))
        (:`OnCompleted`
          (set `CharacterMovementComponent.GroundFriction` (`self.OriginalGroundFrictionFromBP_VAL`) _charactermovement :!label _label)
          (bind _characterbase_2 (`self.Get Player Character and Controller`))
          (`/Game/ThirdPerson/Blueprints/BP_VAl.SetCollisionToPawn` _characterbase_2 "ECR_Block")
          (`self.K2_EndAbility`))
        (:`OnBlendOut`
          (goto _label))
        (:`OnInterrupted`
          (goto _label))
        (:`OnCancelled`
          (goto _label))))
    (:`CastFailed`
      (`self.K2_EndAbility`))))