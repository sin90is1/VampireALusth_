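; BP_IceBall is the actor for the Ice Ball gameplay ability, delivering a gameplay effect to hostile BP_VAl characters.
; On box overlap, it checks hostility between the hit character and its instigator, then has the instigator apply the ability-provided effect spec to that target.
; It destroys itself after a hostile hit or when its six-second lifetime timer expires.
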(event `self.ReceiveBeginPlay`
  (`KismetSystemLibrary.K2_SetTimerDelegate` (delegate `TimeToDie`) 6.0))

(event `TimeToDie`
  (`self.K2_DestroyActor`))

(event `self.Box.OnComponentBeginOverlap`
  (params (OverlappedComponent :type "PrimitiveComponent Object Reference") (OtherActor :type "Actor Object Reference") (OtherComp :type "PrimitiveComponent Object Reference") (OtherBodyIndex :type Integer) (bFromSweep :type Boolean) (SweepResult :type "HitResult Structure (by ref)"))
  (bind _asbp_val (cast `/Game/ThirdPerson/Blueprints/BP_VAl` OtherActor))
  (bind _asbp_val_2 (cast `/Game/ThirdPerson/Blueprints/BP_VAl` (`self.GetInstigator`)))
  (bind _returnvalue (`VampireALusthCharacter.IsOtherHostile` _asbp_val _asbp_val_2))
  (if _returnvalue
    (`VampireALusthCharacter.ApplyGESpectHandleTargetDataSpecsHandle` _asbp_val_2 (`self.EffectSpectHandleFromAbility`) (`AbilitySystemBlueprintLibrary.AbilityTargetDataFromActor` OtherActor))
    (`self.K2_DestroyActor`)))

(fn `UserConstructionScript`)