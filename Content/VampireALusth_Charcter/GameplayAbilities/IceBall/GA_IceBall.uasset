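; GA_IceBall is a Gameplay Ability that casts an ice ball projectile from the player character.
; It commits, triggers the UI cooldown and plays a slowed cast montage, then waits for the Skill.IceBall.fire gameplay event.
; On that event it spawns BP_IceBall_2 slightly above the character, handing it an outgoing GE_IceBallDamage effect spec.
; The ability ends shortly after firing or whenever the montage finishes or is interrupted.
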(event `self.K2_ActivateAbility`
  (`self.K2_CommitAbility`)
  (`self.DoUICooldown`)
  (`AbilityTask_PlayMontageAndWait.CreatePlayMontageAndWaitProxy` "None" "/Game/VampireALusth_Charcter/Animation/AM_IceBall.AM_IceBall" 0.7
    (:`then`
      (`AbilityTask_WaitGameplayEvent.WaitGameplayEvent` (struct :`TagName` "skill.IceBall.fire") null
        (:`EventReceived`
          (bind _characterbase (`self.Get Player Character and Controller`))
          (bind _returnvalue (`SceneComponent.GetRelativeTransform` (`Actor.RootComponent` _characterbase)))
          (`|SpawnActorFromClass` "/Game/VampireALusth_Charcter/GameplayAbilities/IceBall/BP_IceBall_2.BP_IceBall_2_C" (`KismetMathLibrary.MakeTransform` (`KismetMathLibrary.MakeVector` (.x (.location _returnvalue)) (.y (.location _returnvalue)) (+ (.z (.location _returnvalue)) 50.0)) (.rotation _returnvalue) (.scale _returnvalue)) "AlwaysSpawn" "OverrideRootScale" null (`self.MakeOutgoingGameplayEffectSpec` "/Game/VampireALusth_Charcter/GameplayAbilities/IceBall/GE_IceBallDamage.GE_IceBallDamage_C") _characterbase)
          (`KismetSystemLibrary.Delay` 0.6)
          (`self.K2_EndAbility`))))
    (:`OnCompleted`
      (`self.K2_EndAbility` :!label _label))
    (:`OnBlendOut`
      (goto _label))
    (:`OnInterrupted`
      (goto _label))
    (:`OnCancelled`
      (goto _label))))