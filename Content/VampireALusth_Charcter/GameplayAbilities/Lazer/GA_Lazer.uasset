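; Gameplay ability that casts a channeled laser from the player character, damaging and slowing targets.
; Activation commits, starts UI cooldown and the casting montage, then after a delay attaches BP_Lazer to a mesh socket and enables camera-controlled rotation.
; Damage events apply GE_LazerDamage and reduce BP_VAl walk speed while cost remains affordable.
; Cancel events or exhausted cost end the ability, removing the draining cost effect, laser and rotation lock.
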(event `self.K2_ActivateAbility`
  (`self.K2_CommitAbility`)
  (`self.DoUICooldown`)
  (`AbilityTask_PlayMontageAndWait.CreatePlayMontageAndWaitProxy` "None" "/Game/VampireALusth_Charcter/Animation/AM_LazerCasting.AM_LazerCasting" 0.7
    (:`then`
      (`AbilityTask_WaitGameplayEvent.WaitGameplayEvent` (struct :`TagName` "skill.lazer.cancel") null
        (:`then`
          (`KismetSystemLibrary.Delay` 0.55)
          (bind _characterbase (`self.Get Player Character and Controller`))
          (bind (_asynctaskproxy _spawnedactor) (`AbilityTask_SpawnActor.SpawnActor` (struct) "/Game/VampireALusth_Charcter/GameplayAbilities/Lazer/LazerAssets/BP_Lazer.BP_Lazer_C" _characterbase)
            (:`then`
              (bind _output_get (set `self.LazerActor` _spawnedactor))
              (`Actor.K2_AttachToComponent` _output_get (`Character.Mesh` _characterbase) "Lazer" "SnapToTarget" "SnapToTarget" "KeepRelative" true)
              (`/Game/ThirdPerson/Blueprints/BP_VAl.MakeCamera ControlRotation` _characterbase true)
              (bind (_asynctaskproxy_2 _payload) (`AbilityTask_WaitGameplayEvent.WaitGameplayEvent` (struct :`TagName` "skill.lazer.dealDamage") null)
                (:`EventReceived`
                  (bind _can (`self.IsCostStillAvailable`))
                  (if _can
                    (bind (_eventtag _instigator _target _optionalobject _optionalobject2 _contexthandle _instigatortags _targettags _eventmagnitude _targetdata) (break `GameplayEventData` _payload))
                    (`self.BP_ApplyGameplayEffectToTarget` _targetdata "/Game/VampireALusth_Charcter/GameplayAbilities/Lazer/GE_LazerDamage.GE_LazerDamage_C")
                    (for _array_element (`AbilitySystemBlueprintLibrary.GetActorsFromTargetData` _targetdata)
                      (bind _asbp_val (cast `/Game/ThirdPerson/Blueprints/BP_VAl` _array_element))
                      (`/Game/ThirdPerson/Blueprints/BP_VAl.ReduceWalkSpeed` _asbp_val 50.0))
                    (else
                      (`self.K2_EndAbility`))))))))
        (:`EventReceived`
          (`self.K2_EndAbility`))))))

(event `self.K2_OnEndAbility`
  (params (bWasCancelled :type Boolean))
  (bind _lazeractor (`self.LazerActor`))
  (`self.BP_RemoveGameplayEffectFromOwnerWithAssetTags` (struct :`GameplayTags` (struct :`(TagName` "skill.lazer.drainingCost"))))
  (if (`KismetSystemLibrary.IsValid` _lazeractor)
    (`Actor.K2_DestroyActor` _lazeractor))
  (bind _characterbase (`self.Get Player Character and Controller`))
  (`/Game/ThirdPerson/Blueprints/BP_VAl.MakeCamera ControlRotation` _characterbase false))