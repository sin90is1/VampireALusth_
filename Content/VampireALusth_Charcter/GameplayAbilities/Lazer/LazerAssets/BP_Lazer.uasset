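; Laser hazard actor for the Lazer gameplay ability that tracks hostile BP_VAl characters inside its box.
; Overlap start adds hostiles, as judged by the instigator, and spawns a small effect on them; overlap end removes characters and calls SetBackWalkSpeed on them.
; A looping timer sends the overlap list as target data in a Skill.lazer.dealDamage gameplay event to the instigator, leaving damage application outside this actor.
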(event `self.ReceiveBeginPlay`
  ;[1 1 1] Send Damage Event 0.3 PerSeconds
  (`KismetSystemLibrary.K2_SetTimerDelegate` (delegate `SendDealDamageEvent`) 0.3 true))

(event `SendDealDamageEvent`
  ;[1 1 1] Send Damage Event 0.3 PerSeconds
  (`AbilitySystemBlueprintLibrary.SendGameplayEventToActor` (`self.GetInstigator`) (struct :`TagName` "skill.lazer.dealDamage") (make `GameplayEventData` (struct) null null null null (struct) (struct) (struct) 0.0 (`AbilitySystemBlueprintLibrary.AbilityTargetDataFromActorArray` (`self.OverlapingActors`)))))

(event `self.Box.OnComponentBeginOverlap`
  (params (OverlappedComponent :type "PrimitiveComponent Object Reference") (OtherActor :type "Actor Object Reference") (OtherComp :type "PrimitiveComponent Object Reference") (OtherBodyIndex :type Integer) (bFromSweep :type Boolean) (SweepResult :type "HitResult Structure (by ref)"))
  (bind _asbp_val (cast `/Game/ThirdPerson/Blueprints/BP_VAl` OtherActor))
  (bind _asbp_val_2 (cast `/Game/ThirdPerson/Blueprints/BP_VAl` (`self.GetInstigator`)))
  (bind _returnvalue (`VampireALusthCharacter.IsOtherHostile` _asbp_val_2 _asbp_val))
  (if _returnvalue
    (`KismetArrayLibrary.Array_AddUnique` (`self.OverlapingActors`) _asbp_val)
    (`NiagaraFunctionLibrary.SpawnSystemAtLocation` (`self.NewVar_0`) (`SceneComponent.K2_GetComponentLocation` (`Actor.RootComponent` _asbp_val)) (struct) (0.2 0.2 0.2))))

(event `self.Box.OnComponentEndOverlap`
  (params (OverlappedComponent :type "PrimitiveComponent Object Reference") (OtherActor :type "Actor Object Reference") (OtherComp :type "PrimitiveComponent Object Reference") (OtherBodyIndex :type Integer))
  (bind _asbp_val (cast `/Game/ThirdPerson/Blueprints/BP_VAl` OtherActor))
  (`KismetArrayLibrary.Array_RemoveItem` (`self.OverlapingActors`) _asbp_val)
  (`/Game/ThirdPerson/Blueprints/BP_VAl.SetBackWalkSpeed` _asbp_val false))

(fn `UserConstructionScript`)