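; GA_FireBlast is a gameplay ability that pulls nearby BP_VAl characters toward the owner, then blasts them away with damage.
; It commits, starts the UI cooldown and montage, and immediately gathers actors within 800 units to pull, without waiting on the pull event.
; The montage's push event applies damage and a stunning push to those stored targets, reusing the pull loop's cast for direction.
; The ability ends with the montage.
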(event `self.K2_ActivateAbility`
  (bind _targetdatahandle (`self.TargetDataHandle`))
  (`self.K2_CommitAbility`)
  (`self.DoUICooldown`)
  (`AbilityTask_PlayMontageAndWait.CreatePlayMontageAndWaitProxy` "None" "/Game/VampireALusth_Charcter/Animation/AM_FireBlast.AM_FireBlast" 1.0 "Start"
    (:`then`
      (`AbilityTask_WaitGameplayEvent.WaitGameplayEvent` (struct :`TagName` "skill.fireBlast.pull") null
        (:`then`
          (bind (_asynctaskproxy _data) (`AbilityTask_WaitTargetData.WaitTargetData` "None" "Instant" "/Script/VampireALusth.GATargetActorAround" 800.0 (struct) (struct) null)
            (:`then`
              (`AbilityTask_WaitGameplayEvent.WaitGameplayEvent` (struct :`TagName` "skill.fireBlast.push") null
                (:`EventReceived`
                  (`self.BP_ApplyGameplayEffectToTarget` _targetdatahandle "/Game/VampireALusth_Charcter/GameplayAbilities/FireBlast/GE_FireBlast_Damage.GE_FireBlast_Damage_C")
                  (for _array_element (`AbilitySystemBlueprintLibrary.GetActorsFromTargetData` _targetdatahandle)
                    (bind _asbp_val (cast `/Game/ThirdPerson/Blueprints/BP_VAl` _array_element))
                    (bind _returnvalue (`KismetMathLibrary.Normal` (- (`Actor.K2_GetActorLocation` (`self.GetOwningActorFromActorInfo`)) (`Actor.K2_GetActorLocation` (stale _asbp_val_2)))))
                    (`/Game/ThirdPerson/Blueprints/BP_VAl.PushCharacter` _asbp_val (* _returnvalue (-1.0 -1.0 -1.0)) 2000.0 2.0)))))
            (:`ValidData`
              (set `self.TargetDataHandle` _data)
              (for _array_element_2 (`AbilitySystemBlueprintLibrary.GetActorsFromTargetData` _data)
                (bind _asbp_val_2 (cast `/Game/ThirdPerson/Blueprints/BP_VAl` _array_element_2))
                (`/Game/ThirdPerson/Blueprints/BP_VAl.PushCharacter` _asbp_val_2 _returnvalue 1200.0 3.0)))))))
    (:`OnCompleted`
      (`self.K2_EndAbility` :!label _label))
    (:`OnBlendOut`
      (goto _label))
    (:`OnInterrupted`
      (goto _label))
    (:`OnCancelled`
      (goto _label))))