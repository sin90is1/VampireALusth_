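; BP_GameplayAbilityTarget is a GAS ability with cooldown and cost helpers for the player character, with no activation or targeting logic of its own.
; A helper resolves the owning BP_VAl and its player controller.
; DoUICooldown starts cooldowns on primary UI slots matching the ability class.
; IsCostStillAvailable compares the current Health, Mana or Energy attribute against the negated cost from the ability info.
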(fn `DoUICooldown`
  (bind (_characterbase _playercontroller) (`self.Get Player Character and Controller`))
  (`/Engine/EditorBlueprintResources/StandardMacros.IsValid` _playercontroller
    (:`Is Valid`
      (for _array_element (`/Game/UI/WBP_PrimaryUI.Slots` (`/Game/Blueprints/GameMode/BP_VALPlayerController.PrimaryUI` _playercontroller))
        (bind _returnvalue (`self.GetAbilityInfo`))
        (bind (_ability_info_cooldownduration _ability_info_cost _ability_info_costtype _ability_info_uimat _ability_info_abilityclass) (break `GameplayAbilityInfo` (`/Game/UI/WBP_Ability_Slot.Ability Info` _array_element)))
        (if (== (`.AbilityClass` (break `GameplayAbilityInfo` _returnvalue)) _ability_info_abilityclass)
          (`/Game/UI/WBP_Ability_Slot.StartCooldown` _array_element))))))

(fn `Get Player Character and Controller`
  (returns (CharacterBase :type "/Game/ThirdPerson/Blueprints/BP_VAl Object Reference") (PlayerController :type "/Game/Blueprints/GameMode/BP_VALPlayerController Object Reference"))
  (bind _asbp_val (cast `/Game/ThirdPerson/Blueprints/BP_VAl` (`self.GetOwningActorFromActorInfo`)))
  (bind _asbp_valplayer_controller (cast `/Game/Blueprints/GameMode/BP_VALPlayerController` (`Pawn.GetController` _asbp_val))
    (:`then`
      _)
    (:`CastFailed`
      _))
  (return _asbp_val _asbp_valplayer_controller))

(fn `IsCostStillAvailable`
  (returns (Can :type Boolean))
  (locals (Cost :type "Float (single-precision)"))
  (bind _returnvalue (`self.GetAbilityInfo`))
  (set `local.Cost` (* (`.Cost` (break `GameplayAbilityInfo` _returnvalue)) -1.0))
  (switch `EAbilityCostType` (`.CostType` (break `GameplayAbilityInfo` _returnvalue))
    (:`Health`
      (bind _characterbase (`self.Get Player Character and Controller`))
      (bind (_health_basevalue _health_currentvalue) (break `GameplayAttributeData` (`VampireALusthAttributeSet.Health` (`VampireALusthCharacter.AttributeSet` _characterbase))))
      (return (> _health_currentvalue (`local.Cost`))))
    (:`Mana`
      (bind _characterbase_2 (`self.Get Player Character and Controller`))
      (bind (_mana_basevalue _mana_currentvalue) (break `GameplayAttributeData` (`VampireALusthAttributeSet.Mana` (`VampireALusthCharacter.AttributeSet` _characterbase_2))))
      (return (> _mana_currentvalue (`local.Cost`))))
    (:`Energy`
      (bind _characterbase_3 (`self.Get Player Character and Controller`))
      (bind (_energy_basevalue _energy_currentvalue) (break `GameplayAttributeData` (`VampireALusthAttributeSet.Energy` (`VampireALusthCharacter.AttributeSet` _characterbase_3))))
      (return (> _energy_currentvalue (`local.Cost`))))))