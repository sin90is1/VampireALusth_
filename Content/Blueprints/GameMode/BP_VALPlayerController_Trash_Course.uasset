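; Player controller for the BP_VAl character that creates the primary UI and handles input for look, jump, crouch, sprint, melee and target cancel.
; Six slot inputs look up ability classes in the UI and activate them through the Ability System Component, setting targeting and ending combos.
; Direct movement input is disabled in favor of root motion; the controller instead exposes a sprint-driven movement state and camera-yaw-relative desired direction.
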(event `self.ReceiveBeginPlay`
  (bind _returnvalue (`|CreateWidget` "/Game/UI/WBP_PrimaryUI.WBP_PrimaryUI_C"))
  (bind _output_get (set `self.PrimaryUI` _returnvalue))
  (`UserWidget.AddToViewport` _output_get 0))

(event `InputAction|Melee`
  (params (Key :type "Key Structure"))
  ;[1 1 1] Abilities
  (:`Pressed`
    (bind _asbp_val (cast `/Game/ThirdPerson/Blueprints/BP_VAl` (`self.K2_GetPawn`)))
    (`/Game/ThirdPerson/Blueprints/BP_VAl.Melee` _asbp_val)))

(event `InputAction|Jump`
  (params (Key :type "Key Structure"))
  ;[1 1 1] Basic Controll
  (:`Pressed`
    (if (`self.CanJump`)
      (bind _ascharacter (cast `Character` (`self.K2_GetPawn`)))
      (set `self.CanJump` false)
      (`Character.Jump` _ascharacter)
      (`KismetSystemLibrary.Delay` 0.2)
      (set `self.CanJump` true)))
  (:`Released`
    (bind _ascharacter_2 (cast `Character` (`self.K2_GetPawn`)))
    (`Character.StopJumping` _ascharacter_2)))

(event `self.AddAbilityToUI`
  (params (AbilityInfo :type "GameplayAbilityInfo Structure"))
  ;[1 1 1] Abilities
  (`/Game/UI/WBP_PrimaryUI.AddAbilityToSlot` (`self.PrimaryUI`) AbilityInfo))

(event `InputAction|Cancle`
  (params (Key :type "Key Structure"))
  ;[1 1 1] Abilities
  (:`Pressed`
    (bind _asbp_val (cast `/Game/ThirdPerson/Blueprints/BP_VAl` (`self.K2_GetPawn`)))
    (`AbilitySystemComponent.TargetCancel` (`AbilitySystemBlueprintLibrary.GetAbilitySystemComponent` _asbp_val))))

(event `InputAction|Crouch`
  (params (Key :type "Key Structure"))
  ;[1 1 1] Basic Controll
  (:`Pressed`
    (bind _ascharacter (cast `Character` (`self.K2_GetPawn`)))
    (`Character.Crouch` _ascharacter))
  (:`Released`
    (bind _ascharacter_2 (cast `Character` (`self.K2_GetPawn`)))
    (`Character.UnCrouch` _ascharacter_2)))

(event `InputAction|SlotOneAbility`
  (params (Key :type "Key Structure"))
  ;[1 1 1] Abilities
  (:`Pressed`
    (`self.TryActivateAbilityInUISlot` 0)))

(event `InputAction|SlotFourAbility`
  (params (Key :type "Key Structure"))
  ;[1 1 1] Abilities
  (:`Pressed`
    (`self.TryActivateAbilityInUISlot` 3)))

(event `InputAction|SlotTwoAbility`
  (params (Key :type "Key Structure"))
  ;[1 1 1] Abilities
  (:`Pressed`
    (`self.TryActivateAbilityInUISlot` 1)))

(event `InputAction|SlotFiveAbility`
  (params (Key :type "Key Structure"))
  ;[1 1 1] Abilities
  (:`Pressed`
    (`self.TryActivateAbilityInUISlot` 4)))

(event `InputAction|SlotSixAbility`
  (params (Key :type "Key Structure"))
  ;[1 1 1] Abilities
  (:`Pressed`
    (`self.TryActivateAbilityInUISlot` 5)))

(event `InputAction|SlotThreeAbility`
  (params (Key :type "Key Structure"))
  ;[1 1 1] Abilities
  (:`Pressed`
    (`self.TryActivateAbilityInUISlot` 2)))

(event `InputAxis|Look Up / Down Mouse`
  (params (AxisValue :type "Float (single-precision)"))
  ;[1 1 1] Basic Controll
  (`self.AddPitchInput` AxisValue))

(event `InputAxis|Turn Right / Left Mouse`
  (params (AxisValue :type "Float (single-precision)"))
  ;[1 1 1] Basic Controll
  (`self.AddYawInput` AxisValue))

(event `InputAxis|Look Up / Down Gamepad`
  (params (AxisValue :type "Float (single-precision)"))
  ;[1 1 1] Basic Controll
  (`self.AddPitchInput` AxisValue))

(event `InputAxis|Turn Right / Left Gamepad`
  (params (AxisValue :type "Float (single-precision)"))
  ;[1 1 1] Basic Controll
  (`self.AddYawInput` AxisValue))

(event `InputAction|Sprints`
  (params (Key :type "Key Structure"))
  ;[1 1 1] Basic Controll
  (:`Pressed`
    (set `self.Movement State` "NewEnumerator1"))
  (:`Released`
    (set `self.Movement State` "NewEnumerator0")))

(event `InputAxis|Move Forward / Backward`
  (params (AxisValue :type "Float (single-precision)"))
  ;[1 1 1] Not Using anymore cuz of rootmotion but scared to delet even when I have a copy
)

(event `InputAxis|Move Right / Left`
  (params (AxisValue :type "Float (single-precision)"))
  ;[1 1 1] Not Using anymore cuz of rootmotion but scared to delet even when I have a copy
)

(fn `Get Desired Velocity`
  (returns (DesigredVelocity :type "Vector Structure"))
  (bind (_returnvalue_roll _returnvalue_pitch _returnvalue_yaw) (`KismetMathLibrary.BreakRotator` (`Pawn.GetControlRotation` (`GameplayStatics.GetPlayerPawn` 0))))
  (return (`KismetMathLibrary.Normal` (+ (* (`KismetMathLibrary.GetForwardVector` (`KismetMathLibrary.MakeRotator` 0.0 0.0 _returnvalue_yaw)) (`self.GetInputAxisValue`)) (* (`KismetMathLibrary.GetRightVector` (`KismetMathLibrary.MakeRotator` 0.0 0.0 _returnvalue_yaw)) (`self.GetInputAxisValue`))))))

(fn `Get Movement State`
  (returns (MovementState :type "/Game/Blueprints/GameMode/MovementState Enum"))
  (return (`self.Movement State`)))

(fn `TryActivateAbilityInUISlot`
  (params (SlotNumber :type Integer))
  (bind (_abilityclass _valid) (`/Game/UI/WBP_PrimaryUI.GetSlotAbilityClass` (`self.PrimaryUI`) SlotNumber))
  (if _valid
    (bind _asbp_val (cast `/Game/ThirdPerson/Blueprints/BP_VAl` (`self.K2_GetPawn`)))
    (`AbilitySystemComponent.TryActivateAbilityByClass` (`AbilitySystemBlueprintLibrary.GetAbilitySystemComponent` _asbp_val) _abilityclass true)
    (castclass `/Game/VampireALusth_Charcter/GameplayAbilities/BP_GameplayAbilityTarget` _abilityclass
      (:`then`
        (set `/Game/ThirdPerson/Blueprints/BP_VAl.Targeting` true _asbp_val))
      (:`CastFailed`
        (set `/Game/ThirdPerson/Blueprints/BP_VAl.Targeting` false _asbp_val)))
    (`/Game/ThirdPerson/Blueprints/BP_VAl.EndCombo` _asbp_val)))

(fn `UserConstructionScript`)